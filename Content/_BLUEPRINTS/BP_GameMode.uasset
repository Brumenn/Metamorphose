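; Game mode for a timed Red vs Blue local multiplayer match that creates players and shows a countdown on BeginPlay.
; Tick counts down the clock, then shows the winner or tie widget, disables the first player's input and slows time.
; Tick also fires blizzard, meteor and wave hazards through a random MultiGate, with delays shortened by a difficulty timeline scaled to match length.
; The respawn and game-over logic is disconnected.
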(event `self.ReceiveTick`
  (params (DeltaSeconds :type "Float (single-precision)"))
  (bind _returnvalue (`GameplayStatics.GetPlayerController` 0))
  (bind _returnvalue_2 (`Controller.K2_GetPawn` _returnvalue))
  ;[1 1 1] Scoring and Winners
  (if (not (`self.gameFinished`))
    (`|ExecutionSequence`
      (:`then_0`
        (`KismetSystemLibrary.Delay` 1.0)
        (if (not (`self.gameFinished`))
          (set `self.Seconds` (- (`self.Seconds`) 1))
          (if (< (`self.Seconds`) 0)
            (set `self.Minutes` (- (`self.Minutes`) 1))
            (set `self.Seconds` 59))
          (if (== (`self.Seconds`) 0)
            (if (== (`self.Minutes`) 0)
              (if (== (`self.BlueScore`) (`self.RedScore`))
                (bind _returnvalue_3 (`|CreateWidget` "/Game/_HUDS/SCORE/HUD_Equality.HUD_Equality_C"))
                (`UserWidget.AddToViewport` _returnvalue_3 0)
                (elif (> (`self.BlueScore`) (`self.RedScore`))
                  (bind _returnvalue_4 (`|CreateWidget` "/Game/_HUDS/SCORE/HUD_Blu_Wins.HUD_Blu_Wins_C"))
                  (`UserWidget.AddToViewport` _returnvalue_4 0)
                  (else
                    (bind _returnvalue_5 (`|CreateWidget` "/Game/_HUDS/SCORE/HUD_RED_Wins.HUD_RED_Wins_C"))
                    (`UserWidget.AddToViewport` _returnvalue_5 0))))
              (`WidgetBlueprintLibrary.SetInputMode_GameAndUIEx` _returnvalue null)
              (set `PlayerController.bShowMouseCursor` true _returnvalue)
              (`/Engine/EditorBlueprintResources/StandardMacros.IsValid` _returnvalue_2
                (:`Is Valid`
                  (`self.DisableInput` _returnvalue_2 _returnvalue)
                  (set `self.gameFinished` true)
                  (`GameplayStatics.SetGlobalTimeDilation` 0.2)))))))
      (:`then_1`
        ;[1 1 1] TICK / EVENTS -Randomise
        (`/Engine/EditorBlueprintResources/StandardMacros.IsValid` (`Controller.K2_GetPawn` (`GameplayStatics.GetPlayerController` 0))
          (:`Is Valid`
            (`|MultiGate` true true :!label _label
              (:`Out 0`
                (`KismetSystemLibrary.Delay` (`KismetMathLibrary.RandomFloatInRange` 4.0 (`KismetMathLibrary.Lerp` 10.0 6.0 (`self.DifficultyAmount`))))
                (if (not (`self.gameFinished`))
                  (`/Game/_BLUEPRINTS/BLIZZARD/BP_Blizzard.EVENT_Blizzard` (`self.Blizzard_Ref`))
                  (goto _label :!via `Reset`)))
              (:`Out 1`
                (`KismetSystemLibrary.Delay` (`KismetMathLibrary.RandomFloatInRange` 0.5 (`KismetMathLibrary.Lerp` 3.0 0.5 (`self.DifficultyAmount`))))
                (if (not (`self.gameFinished`))
                  (`/Game/_BLUEPRINTS/BP_MeteorTracer.SpawnMeteorEvent` (`self.Meteor_Ref`))
                  (goto _label :!via `Reset`)))
              (:`Out 2`
                (`KismetSystemLibrary.Delay` (`KismetMathLibrary.RandomFloatInRange` 4.0 (`KismetMathLibrary.Lerp` 9.0 5.0 (`self.DifficultyAmount`))))
                (if (not (`self.gameFinished`))
                  (`/Game/_BLUEPRINTS/VAGUE/BP_VAGUE.EVENT_Wave` (`self.Vague_Ref`))
                  (goto _label :!via `Reset`))))))))))

(event `SpawnCharacter`
  (params (PlayerController :type "PlayerController Object Reference"))
  ;[1 1 1] Spawn Character
)

(event `self.ReceiveBeginPlay`
  (bind _numberofplayers (`self.NumberOfPLayers`))
  ;[0.5938 0.5938 0.5938] BEGIN PLAY Settings
  (set `self.IsBeginPlay?` true)
  (`|ExecutionSequence`
    (:`then_0`
      (bind _returnvalue (`|CreateWidget` "/Game/_HUDS/Countdown.Countdown_C"))
      (`UserWidget.AddToViewport` _returnvalue 0))
    (:`then_1`
      ;[0.5938 0.5938 0.5938] Create Players
      (bind _outactors (`GameplayStatics.GetAllActorsOfClass` "/Script/Engine.PlayerStart"))
      (set `self.SpawnPoints` _outactors)
      (while (<= _numberofplayers 3)
        (set `self.NumberOfPLayers` (+ _numberofplayers 1))
        (`GameplayStatics.CreatePlayer` -1)))
    (:`then_2`
      ;[1 1 1] REFS - Events
      (bind _outactors_2 (`GameplayStatics.GetAllActorsOfClass` "/Game/_BLUEPRINTS/BLIZZARD/BP_Blizzard.BP_Blizzard_C"))
      (set `self.Blizzard_Ref` (`|GetArrayItem` _outactors_2))
      (bind _outactors_3 (`GameplayStatics.GetAllActorsOfClass` "/Game/_BLUEPRINTS/BP_MeteorTracer.BP_MeteorTracer_C"))
      (set `self.Meteor_Ref` (`|GetArrayItem` _outactors_3))
      (bind _outactors_4 (`GameplayStatics.GetAllActorsOfClass` "/Game/_BLUEPRINTS/VAGUE/BP_VAGUE.BP_VAGUE_C"))
      (set `self.Vague_Ref` (`|GetArrayItem` _outactors_4))
      (bind _asbp_player_controller (cast `/Game/_BLUEPRINTS/BP_PlayerController` (`GameplayStatics.GetPlayerController` 0)))
      (set `self.BP_PC_REF` _asbp_player_controller))
    (:`then_3`
      ;[1 1 1] Increase variable difficulty during level thanks to timeline
      (`TimelineComponent.SetPlayRate` (`self.EventTimeline`) (/ 1.0 (`KismetMathLibrary.Conv_IntToDouble` (+ (* (`self.Minutes`) 60) (`self.Seconds`)))))
      (bind (_direction _value_0_to_1) (`Timeline|EventTimeline` :!via `PlayFromStart`)
        (:`Update`
          (set `self.DifficultyAmount` _value_0_to_1))))))

(fn `UserConstructionScript`)