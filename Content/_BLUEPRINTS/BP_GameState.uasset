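; BP_GameState is a game-state Blueprint that caches references to the rabbit, bird and pig characters on BeginPlay.
; OnHit prints a test message and contains a recursive red/white sprite flash using delays, meant to stop at RedSpriteMax.
; The flash sits behind a DoN with a count of zero, so it never runs as wired.
; When RedSpriteEnable is false, OnHit resets the sprite to white; DestroyActor is empty.
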(event `self.ReceiveBeginPlay`
  (`|ExecutionSequence`
    (:`then_0`
      (bind _outactors (`GameplayStatics.GetAllActorsOfClass` "/Game/_CHAR/_HEROES/1_RABBIT/1_Char_RABBIT.1_Char_RABBIT_C"))
      (set `self.1_Rabbit_Ref` (`|GetArrayItem` _outactors)))
    (:`then_1`
      (bind _outactors_2 (`GameplayStatics.GetAllActorsOfClass` "/Game/_CHAR/_HEROES/2_BIRD/2_Char_BIRD_2.2_Char_BIRD_2_C"))
      (set `self.2_Bird_Ref` (`|GetArrayItem` _outactors_2)))
    (:`then_2`
      (bind _outactors_3 (`GameplayStatics.GetAllActorsOfClass` "/Game/_CHAR/_HEROES/3_PIG/3_Char_PIG.3_Char_PIG_C"))
      (set `self.3_Pig_Ref` (`|GetArrayItem` _outactors_3)))))

(event `DestroyActor`)

(event `OnHit`
  (bind _spriteref (`self.SpriteREF`))
  ;[1 1 1] test
  (`KismetSystemLibrary.PrintString` "HIT")
  (if (`self.RedSpriteEnable`)
    (bind _counter (`/Engine/EditorBlueprintResources/StandardMacros.Do N` 0)
      (:`Exit`
        (`PaperFlipbookComponent.SetSpriteColor` _spriteref (struct :`R` 0.416667 :`B` 0.0073 :`A` 1.0))
        (set `self.RedSprit_Current` _counter)
        (`KismetSystemLibrary.Delay` (`self.RedSpriteColor_Time`))
        (`PaperFlipbookComponent.SetSpriteColor` _spriteref (struct :`R` 1.0 :`G` 1.0 :`B` 1.0 :`A` 1.0))
        (`KismetSystemLibrary.Delay` (`self.RedSpriteColor_Time`))
        (`self.OnHit`)
        (if (== (`self.RedSprit_Current`) (`self.RedSprite_Max`))
          (set `self.RedSpriteEnable` false))))
    (else
      (`PaperFlipbookComponent.SetSpriteColor` _spriteref (struct :`R` 1.0 :`G` 1.0 :`B` 1.0 :`A` 1.0)))))

(fn `UserConstructionScript`)