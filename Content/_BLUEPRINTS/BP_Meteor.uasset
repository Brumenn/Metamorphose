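; BP_Meteor is a projectile actor that flies from its start position to TargetPos and explodes on impact.
; A timeline, with play rate set by Speed, lerps its location without sweeping.
; When its sphere overlaps a StaticMeshActor, it shakes the first player's camera, spawns BP_MeteorExplosion, then destroys ParentObject and itself.
; An ApplyPointDamage node is unconnected, so the meteor applies no damage itself.
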(event `self.ReceiveBeginPlay`
  ;[1 1 1] Store position value
  (set `self.sourcePos` (`self.K2_GetActorLocation` self))
  ;[1 1 1] Timeline scaling
  (`TimelineComponent.SetPlayRate` (`self.MovementTimeline`) (`self.speed`))
  (bind (_direction _value_0_to_1) (`Timeline|MovementTimeline` :!via `PlayFromStart`)
    (:`Update`
      ;[1 1 1] Update trajectory
      (`self.K2_SetActorLocation` self (`KismetMathLibrary.VLerp` (`self.sourcePos`) (`self.targetPos`) _value_0_to_1) false false))))

(event `self.Sphere.OnComponentBeginOverlap`
  (params (OverlappedComponent :type "PrimitiveComponent Object Reference") (OtherActor :type "Actor Object Reference") (OtherComp :type "PrimitiveComponent Object Reference") (OtherBodyIndex :type Integer) (bFromSweep :type Boolean) (SweepResult :type "HitResult Structure (by ref)"))
  (cast `StaticMeshActor` OtherActor)
  (`|ExecutionSequence`
    (:`then_0`
      (`PlayerController.ClientStartCameraShake` :`self` (`GameplayStatics.GetPlayerController` 0) :`Shake` "/Game/_BLUEPRINTS/METEOR/CameraShake_Meteor.CameraShake_Meteor_C" :`Scale` 20.0))
    (:`then_1`
      ;[1 1 1] Spawn Explosion on Overlap
      (`|SpawnActorFromClass` "/Game/_BLUEPRINTS/BP_MeteorExplosion.BP_MeteorExplosion_C" (`KismetMathLibrary.Conv_VectorToTransform` (`self.K2_GetActorLocation`)) "Undefined" "OverrideRootScale" null null)
      (`|ExecutionSequence`
        (:`then_0`
          (`self.K2_DestroyActor` (`self.parentObject`)))
        (:`then_1`
          (`self.K2_DestroyActor`))))))

(fn `UserConstructionScript`)