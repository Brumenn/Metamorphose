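; BP_MeteorExplosion is a self-destroying meteor explosion effect with a physics impulse, fire, flipbook sprite and point light.
; On BeginPlay it fires the force component's impulse, then hides the flipbook shortly afterward.
; After a longer delay it deactivates the fire and runs a timeline that scales the light's current intensity each update, then destroys the actor.
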(event `self.ReceiveBeginPlay`
  (bind _pointlight (`self.PointLight`))
  (`RadialForceComponent.FireImpulse` (`self.ForceComponent`))
  (`|ExecutionSequence`
    (:`then_0`
      (`KismetSystemLibrary.Delay` 5.0)
      (`|ExecutionSequence`
        (:`then_0`
          (`ActorComponent.Deactivate` (`self.Fire`))
          (`KismetSystemLibrary.Delay` 2.5)
          (`self.K2_DestroyActor`))
        (:`then_1`
          (bind (_direction _intensity) (`Timeline|IntensityAnimation`)
            (:`Update`
              (`LightComponent.SetIntensity` _pointlight (`KismetMathLibrary.Lerp` 0.0 (`LightComponentBase.Intensity` _pointlight) _intensity)))))))
    (:`then_1`
      (`KismetSystemLibrary.Delay` 0.5)
      (`SceneComponent.SetVisibility` (`self.PaperFlipbook`) false false))))

(fn `UserConstructionScript`)