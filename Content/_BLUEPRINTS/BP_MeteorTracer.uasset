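; BP_MeteorTracer is an actor that picks a random impact point for a meteor and spawns a BP_MeteorTarget there on BeginPlay.
; LineTraceFromComponent casts a Visibility trace from the root along its forward vector, with the X component replaced by a random value to scatter the direction.
; SpawnMeteorEvent spawns the target at the hit location, or immediately calls itself again on a miss, with no delay or retry limit.
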(event `self.ReceiveBeginPlay`
  (`self.SpawnMeteorEvent`))

(event `SpawnMeteorEvent`
  (bind _defaultsceneroot (`self.DefaultSceneRoot`))
  (bind (_return _outhit) (`self.LineTraceFromComponent` _defaultsceneroot _defaultsceneroot 3000.0))
  (if _return
    (set `self.HitLocation` (`.Location` (`GameplayStatics.BreakHitResult` _outhit)))
    (`|SpawnActorFromClass` "/Game/_BLUEPRINTS/BP_MeteorTarget.BP_MeteorTarget_C" (`KismetMathLibrary.Conv_VectorToTransform` (`self.HitLocation`)) "Undefined" "OverrideRootScale" null null)
    (else
      (`self.SpawnMeteorEvent`))))

(fn `LineTraceFromComponent`
  (params (StartComponent :type "SceneComponent Object Reference") (EndComponent :type "SceneComponent Object Reference") (Lenght :type "Float (double-precision)"))
  (returns (Return :type Boolean) (OutHit :type "HitResult Structure"))
  (bind _returnvalue (`SceneComponent.K2_GetComponentLocation` StartComponent))
  (bind (_outhit _returnvalue_2) (`KismetSystemLibrary.LineTraceSingle` _returnvalue (+ (* (`KismetMathLibrary.MakeVector` (`KismetMathLibrary.RandomFloatInRange` -2.0 2.0) (.y (`SceneComponent.GetForwardVector` EndComponent)) (.z (`SceneComponent.GetForwardVector` EndComponent))) Lenght) _returnvalue) "TraceTypeQuery1"))
  (return _returnvalue_2 _outhit))

(fn `UserConstructionScript`)