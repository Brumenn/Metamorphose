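; Player controller that lets the player switch between rabbit, bird and pig pawns, and manages HUD, pause and lives.
; Switching destroys the pawn, spawns and possesses the new one in place, with flags blocking the current form, then restores the level's CAM view.
; Pausing toggles a menu in EventGraph; the PauseGame/UnPauseGame functions are empty.
; Hits rebuild the HUD; lives below zero trigger game over with slow motion.
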(event `PauseButtonPressed`
  (bind _returnvalue (`GameplayStatics.GetPlayerController` 0))
  (bind _returnvalue_2 (`GameplayStatics.GetPlayerController` 0))
  ;[1 1 1] PauseGame
  (`/Engine/EditorBlueprintResources/StandardMacros.IsValid` (`self.PauseMenuRef`) :!label _label
    (:`Is Valid`
      (`Widget.RemoveFromParent` (`self.PauseMenuRef`))
      (`WidgetBlueprintLibrary.SetInputMode_GameOnly` _returnvalue)
      (set `PlayerController.bShowMouseCursor` false _returnvalue)
      (`self.EnableInput` (`self.K2_GetPawn` _returnvalue) _returnvalue)
      (`GameplayStatics.SetGamePaused` false)
      (set `self.PauseMenuRef` null))
    (:`Is Not Valid`
      (bind _returnvalue_3 (`|CreateWidget` "/Game/_HUDS/MENU/PAUSE_MENU.PAUSE_MENU_C"))
      (bind _output_get (set `self.PauseMenuRef` _returnvalue_3))
      (`UserWidget.AddToViewport` _output_get 0)
      (`WidgetBlueprintLibrary.SetInputMode_GameAndUIEx` _returnvalue_2 null)
      (set `PlayerController.bShowMouseCursor` true _returnvalue_2)
      (`self.DisableInput` (`self.K2_GetPawn` _returnvalue_2) _returnvalue_2)
      (`GameplayStatics.SetGamePaused` true))))

(event `InputAction|Pause` :paused true
  (params (Key :type "Key Structure"))
  ;[1 1 1] PauseGame
  (:`Pressed`
    (goto _label)))

(event `self.ReceiveBeginPlay`
  ;[1 1 1] EVENT BEGIN PLAY
  ;;[1 0 0] BEGIN PLAY
  (set `self.bShowMouseCursor` false)
  (`|ExecutionSequence`
    (:`then_1`
      ;;[1 1 1] Get PlayerStart
      (bind _outactors (`GameplayStatics.GetAllActorsOfClass` "/Script/Engine.PlayerStart"))
      (set `self.SpawnPoints` _outactors))
    (:`then_2`
      ;;[1 1 1] Game Mode Ref
      (bind _asbp_game_mode (cast `/Game/_BLUEPRINTS/BP_GameMode` (`GameplayStatics.GetGameMode`)))
      (set `self.GameModeRef` _asbp_game_mode))
    (:`then_3`
      (`self.Create_GameHUD`))
    (:`then_4`
      ;;[0.3061 0.3736 1] Spawn Character/ Set Camera
      (`self.SpawnBeginPlay`)
      (`self.SetCamera`)
      ;;[1 1 1] Set Variables
      (set `self.SpawnEnable?` false)
      (set `self.IsRabbit?` true)
      (set `self.IsPig?` true))))

(event `Create_GameHUD`
  ;[1 1 1] EVENT BEGIN PLAY
  ;;[1 1 1] Game HUD Ref
  (bind _returnvalue (`|CreateWidget` "/Game/_HUDS/MENU/GAME_HUD.GAME_HUD_C" (`GameplayStatics.GetPlayerController` 0)))
  (bind _output_get (set `self.GameHUD_Ref` _returnvalue))
  (`UserWidget.AddToViewport` _output_get 0))

(event `PC_Hit_RemoveLife`
  ;[1 1 1] Remove Life / Game Over
  (bind _output_get (set `self.PC_CurrentLifes` (- (`self.PC_CurrentLifes`) 1)))
  (`KismetSystemLibrary.PrintString` (`KismetStringLibrary.Conv_IntToString` _output_get) true true (struct :`R` 1.0 :`B` 0.125788 :`A` 1.0))
  (`WidgetLayoutLibrary.RemoveAllWidgets`)
  (`self.Create_GameHUD`)
  (if (<= _output_get -1)
    (`self.GameOver`)))

(event `InputAction|Test`
  (params (Key :type "Key Structure"))
  ;[1 1 1] Remove Life / Game Over
)

(event `SetCamera`
  ;[1 1 1] Set Camera's view Target with Blend
  (bind _outactors (`GameplayStatics.GetAllActorsOfClass` "/Game/_CAMERAS/CAM.CAM_C"))
  (set `self.CAM_Ref` (`|GetArrayItem` _outactors))
  (`self.SetViewTargetWithBlend` (`GameplayStatics.GetPlayerController` 0) (`self.CAM_Ref`) 0.0 "VTBlend_Linear" 0.0 false))

(event `InputAction|Spawn_Light`
  (params (Key :type "Key Structure"))
  (bind _returnvalue (`GameplayStatics.GetPlayerController` 0))
  (bind _returnvalue_2 (`self.K2_GetPawn` _returnvalue))
  ;[0.1238 0.7371 1] SPAWN_RABBIT
  (:`Pressed`
    (if (`self.IsRabbit?`)
      (`KismetSystemLibrary.PrintString` "")
      (set `self.PawnTransform` (`self.GetTransform` _returnvalue_2))
      (`self.K2_DestroyActor` _returnvalue_2)
      (bind _returnvalue_3 (`|SpawnActorFromClass` "/Game/_CHAR/_HEROES/1_RABBIT/1_Rabbit.1_Rabbit_C" (`self.PawnTransform`) "AdjustIfPossibleButAlwaysSpawn" "OverrideRootScale" null null))
      (`self.Possess` _returnvalue _returnvalue_3)
      (`self.SetCamera`)
      (set `self.IsRabbit?` false)
      (set `self.IsBird?` true)
      (set `self.IsPig?` true))))

(event `InputAction|Spawn_Medium`
  (params (Key :type "Key Structure"))
  (bind _returnvalue (`GameplayStatics.GetPlayerController` 0))
  (bind _returnvalue_2 (`self.K2_GetPawn` _returnvalue))
  ;[1 0.1771 0.1771] SPAWN_BIRD
  (:`Pressed`
    (if (`self.IsBird?`)
      (`KismetSystemLibrary.PrintString` "")
      (set `self.PawnTransform` (`self.GetTransform` _returnvalue_2))
      (`self.K2_DestroyActor` _returnvalue_2)
      (bind _returnvalue_3 (`|SpawnActorFromClass` "/Game/_CHAR/_HEROES/2_BIRD/0_BASE_Bird.0_BASE_Bird_C" (`self.PawnTransform`) "AdjustIfPossibleButAlwaysSpawn" "OverrideRootScale" null null))
      (`self.Possess` _returnvalue _returnvalue_3)
      (`self.SetCamera`)
      (set `self.IsRabbit?` true)
      (set `self.IsBird?` false)
      (set `self.IsPig?` true))))

(event `InputAction|Spawn_Heavy`
  (params (Key :type "Key Structure"))
  (bind _returnvalue (`GameplayStatics.GetPlayerController` 0))
  (bind _returnvalue_2 (`self.K2_GetPawn` _returnvalue))
  ;[0.9941 1 0.1976] SPAWN_PIG
  (:`Pressed`
    (if (`self.IsPig?`)
      (`KismetSystemLibrary.PrintString` "")
      (set `self.PawnTransform` (`self.GetTransform` _returnvalue_2))
      (`self.K2_DestroyActor` _returnvalue_2)
      (bind _returnvalue_3 (`|SpawnActorFromClass` "/Game/_CHAR/_HEROES/3_PIG/3_Pig.3_Pig_C" (`self.PawnTransform`) "AdjustIfPossibleButAlwaysSpawn" "OverrideRootScale" null null))
      (`self.Possess` _returnvalue _returnvalue_3)
      (`self.SetCamera`)
      (set `self.IsRabbit?` true)
      (set `self.IsBird?` true)
      (set `self.IsPig?` false))))

(event `SpawnBeginPlay`
  (bind _returnvalue (`GameplayStatics.GetPlayerController` 0))
  ;[0.3448 0.1083 0.3542] Spawn Begin PLay
  (if (`self.IsBird?`)
    (`KismetSystemLibrary.PrintString` "")
    (set `self.PawnTransform` (`self.GetTransform` (`|GetArrayItem` (`self.SpawnPoints`))))
    (`self.K2_DestroyActor` (`self.K2_GetPawn` _returnvalue))
    (bind _returnvalue_2 (`|SpawnActorFromClass` "/Game/_CHAR/_HEROES/2_BIRD/0_BASE_Bird.0_BASE_Bird_C" (`self.PawnTransform`) "AdjustIfPossibleButAlwaysSpawn" "OverrideRootScale" null null))
    (`self.Possess` _returnvalue _returnvalue_2)
    (`self.SetCamera`)
    (set `self.IsRabbit?` true)
    (set `self.IsBird?` false)
    (set `self.IsPig?` true)))

(fn `GameOver`
  (bind _returnvalue (`GameplayStatics.GetPlayerController` 0))
  (bind _returnvalue_2 (`self.K2_GetPawn` _returnvalue))
  (bind _returnvalue_3 (`|CreateWidget` "/Game/_HUDS/MENU/GAME_OVER.GAME_OVER_C"))
  (`UserWidget.AddToViewport` _returnvalue_3 0)
  (`WidgetBlueprintLibrary.SetInputMode_GameAndUIEx` _returnvalue null)
  (set `PlayerController.bShowMouseCursor` true _returnvalue)
  (`/Engine/EditorBlueprintResources/StandardMacros.IsValid` _returnvalue_2
    (:`Is Valid`
      (`self.DisableInput` _returnvalue_2 _returnvalue)
      (`GameplayStatics.SetGlobalTimeDilation` 0.2)
      (`self.K2_DestroyActor`))))

(fn `PauseGame`)

(fn `UnPauseGame`)

(fn `UserConstructionScript`)