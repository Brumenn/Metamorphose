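; BP_MeteorExplosion is a timed meteor explosion effect that removes itself.
; On BeginPlay it caches the game state, fires a force impulse, and hides its flipbook shortly after.
; After the set duration it deactivates the fire, destroys the sphere, runs a timeline that drives light intensity, then destroys the actor.
; The sphere overlap only casts to PaperCharacter, with no follow-up logic.
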(event `self.ReceiveBeginPlay`
  (bind _pointlight (`self.PointLight`))
  (`|ExecutionSequence`
    (:`then_0`
      (bind _asbp_game_state (cast `/Game/_BLUEPRINTS/BP_GameState` (`GameplayStatics.GetGameState`)))
      (set `self.GameStateREF` _asbp_game_state))
    (:`then_1`
      (`RadialForceComponent.FireImpulse` (`self.ForceComponent`))
      (`|ExecutionSequence`
        (:`then_0`
          (`KismetSystemLibrary.Delay` (`self.Duration`))
          (`|ExecutionSequence`
            (:`then_0`
              (`ActorComponent.Deactivate` (`self.Fire`))
              (`KismetSystemLibrary.Delay` 2.5)
              (`self.K2_DestroyActor`))
            (:`then_1`
              (bind (_direction _intensity) (`Timeline|IntensityAnimation`)
                (:`Update`
                  (`LightComponent.SetIntensity` _pointlight (`KismetMathLibrary.Lerp` 0.0 (`LightComponentBase.Intensity` _pointlight) _intensity)))))
            (:`then_2`
              (`ActorComponent.K2_DestroyComponent` (`self.Sphere`)))))
        (:`then_1`
          (`KismetSystemLibrary.Delay` 0.5)
          (`SceneComponent.SetVisibility` (`self.PaperFlipbook`) false false))))))

(event `self.Sphere.OnComponentBeginOverlap`
  (params (OverlappedComponent :type "PrimitiveComponent Object Reference") (OtherActor :type "Actor Object Reference") (OtherComp :type "PrimitiveComponent Object Reference") (OtherBodyIndex :type Integer) (bFromSweep :type Boolean) (SweepResult :type "HitResult Structure (by ref)"))
  (cast `PaperCharacter` OtherActor))

(fn `UserConstructionScript`)