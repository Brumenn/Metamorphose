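; BP_MeteorTarget is a meteor impact point that launches a BP_Meteor at its own location and shows a danger zone plane.
; BeginPlay and the Respawn event spawn the meteor high above at a random X offset, passing Speed, the target position and itself as parent.
; The plane's pitch is then derived from a look-at rotation toward the new meteor, mirrored by yaw, so the zone angles with the incoming path.
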(event `Respawn`
  (bind _returnvalue (`self.K2_GetActorLocation`))
  (bind _returnvalue_2 (`|SpawnActorFromClass` "/Game/_BLUEPRINTS/METEOR/BP_Meteor.BP_Meteor_C" (`KismetMathLibrary.Conv_VectorToTransform` (+ (`KismetMathLibrary.MakeVector` (`KismetMathLibrary.RandomFloatInRange` -2500.0 2500.0) 0.0 5000.0) _returnvalue)) "Undefined" "OverrideRootScale" null (`self.speed`) _returnvalue self null :!label _label))
  ;[1 1 1] Look at Zone Danger (Plane)
  (if (< (.yaw (`KismetMathLibrary.FindLookAtRotation` (`SceneComponent.K2_GetComponentLocation` (`self.Plane`)) (`self.K2_GetActorLocation` _returnvalue_2))) 90.0)
    (bind _returnvalue_3 (+ (.pitch (`KismetMathLibrary.FindLookAtRotation` (`SceneComponent.K2_GetComponentLocation` (`self.Plane`)) (`self.K2_GetActorLocation` _returnvalue_2))) -90.0))
    (set `self.angleZone` _returnvalue_3)
    (else
      (bind _output_get (set `self.angleZone` (* -1.0 _returnvalue_3)))))
  (`SceneComponent.K2_SetWorldRotation` (`self.Plane`) (`KismetMathLibrary.MakeRotator` 180.0 _output_get) false false))

(event `self.ReceiveBeginPlay`
  (goto _label))

(fn `UserConstructionScript`)