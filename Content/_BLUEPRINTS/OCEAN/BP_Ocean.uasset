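; BP_Ocean is an ocean actor that moves from its starting position to a target position over the match countdown, acting as the water level.
; On BeginPlay it sets a timeline's play rate from BP_GameMode's minutes and seconds, so the movement spans the timer.
; Each update, unless the game has finished, it lerps the actor's location and pushes a remapped water level to the Countdown HUD widgets.
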(event `self.ReceiveBeginPlay`
  ;[1 1 1] Store position value
  (set `self.sourcePos` (`self.K2_GetActorLocation` self))
  ;[1 1 1] Timeline setup with GM timer synchronization
  (bind _asbp_game_mode (cast `/Game/_BLUEPRINTS/BP_GameMode` (`GameplayStatics.GetGameMode`)))
  (`TimelineComponent.SetPlayRate` (`self.Movement Timeline`) (/ 1.0 (`KismetMathLibrary.Conv_IntToDouble` (+ (* (`/Game/_BLUEPRINTS/BP_GameMode.Minutes` _asbp_game_mode) 60) (`/Game/_BLUEPRINTS/BP_GameMode.Seconds` _asbp_game_mode)))))
  (bind (_direction _value_0_to_1) (`Timeline|Movement Timeline` :!via `PlayFromStart`)
    (:`Update`
      ;[1 1 1] Update z location
      (bind _asbp_game_mode_2 (cast `/Game/_BLUEPRINTS/BP_GameMode` (`GameplayStatics.GetGameMode`)))
      (if (not (`/Game/_BLUEPRINTS/BP_GameMode.gameFinished` _asbp_game_mode_2))
        (`self.K2_SetActorLocation` self (`KismetMathLibrary.VLerp` (`self.sourcePos`) (`self.targetPos`) _value_0_to_1) false false)
        ;[1 1 1] Update HUD Water level
        (bind _foundwidgets (`WidgetBlueprintLibrary.GetAllWidgetsOfClass` "/Game/_HUDS/Countdown.Countdown_C"))
        (`/Game/_HUDS/Countdown.Update_Water_Level` _foundwidgets (`KismetMathLibrary.Lerp` 0.1 0.92 _value_0_to_1))))))

(fn `UserConstructionScript`)