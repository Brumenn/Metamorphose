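; BP_VAGUE is an actor with a VAGUE2 component, apparently a wave hazard (French "vague"), that slides when triggered.
; The VAGUE_Move event uses MoveComponentTo to move the component to a far relative Y position over a few seconds.
; Tick and the component hit event are empty.
; Disconnected leftover nodes would stop the rabbit character, slow time, teleport the wave away or destroy the actor, but never run.
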(event `self.ReceiveTick`
  (params (DeltaSeconds :type "Float (single-precision)")))

(event `VAGUE_Move`
  (`KismetSystemLibrary.MoveComponentTo` (`self.VAGUE2`) (0.0 15000.0 0.0) (struct) false false 8.0))

(event `self.VAGUE2.OnComponentHit`
  (params (HitComponent :type "PrimitiveComponent Object Reference") (OtherActor :type "Actor Object Reference") (OtherComp :type "PrimitiveComponent Object Reference") (NormalImpulse :type "Vector Structure") (Hit :type "HitResult Structure (by ref)")))

(fn `UserConstructionScript`)