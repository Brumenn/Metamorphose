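; BP_Camera_Multi is a shared spring-arm camera that follows up to four player characters.
; Each Tick, a Sequence computes center and longest distance per valid player count, rerunning the shared camera update for each count.
; The Box moves to the center, and the spring arm eases toward it in X/Y with an X offset and fixed starting height.
; Zoom interpolates arm length, but its Max/Min clamp always targets 2500, ignoring distance.
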(event `self.ReceiveBeginPlay`
  ;[1 1 1] Begin Play
  (set `self.CamPosX` (.x (`SceneComponent.K2_GetComponentLocation` (`self.SpringArm`))))
  (set `self.CamPosY` (.y (`SceneComponent.K2_GetComponentLocation` (`self.SpringArm`))))
  (set `self.CamPosStart` (`KismetMathLibrary.MakeVector` 0.0 0.0 (.z (`self.K2_GetActorLocation`)))))

(event `CameraZoom`
  (bind _springarm (`self.SpringArm`))
  ;[1 1 1] Camera Zom
  (set `SpringArmComponent.TargetArmLength` (`KismetMathLibrary.FInterpTo` (`SpringArmComponent.TargetArmLength` _springarm) (`KismetMathLibrary.FMax` (`KismetMathLibrary.FMin` (`self.LongestDistance`) 2000.0) 2500.0) (`self.Delta`) 0.5) _springarm))

(event `self.ReceiveTick`
  (params (DeltaSeconds :type "Float (single-precision)"))
  ;[1 1 1] EVENT TICK
  (`|ExecutionSequence`
    (:`then_0`
      (`/Engine/EditorBlueprintResources/StandardMacros.IsValid` (`GameplayStatics.GetPlayerCharacter` 0)
        (:`Is Valid`
          (`self.Set Longest Distance 1`)
          (`self.Set Center 1`))))
    (:`then_1`
      (`/Engine/EditorBlueprintResources/StandardMacros.IsValid` (`GameplayStatics.GetPlayerCharacter` 1)
        (:`Is Valid`
          (`self.Set Longest Distance 2`)
          (`self.Set Center 2`))))
    (:`then_2`
      (`/Engine/EditorBlueprintResources/StandardMacros.IsValid` (`GameplayStatics.GetPlayerCharacter` 2)
        (:`Is Valid`
          (`self.Set Longest Distance 3`)
          (`self.Set Center 3`))))
    (:`then_3`
      (`/Engine/EditorBlueprintResources/StandardMacros.IsValid` (`GameplayStatics.GetPlayerCharacter` 3)
        (:`Is Valid`
          (`self.Set Longest Distance 4`)
          (`self.Set Center 4`)))))
  (set `self.Delta` DeltaSeconds)
  (`self.CameraZoom`)
  (`self.SetBoxPos`)
  (`self.Set cam Pos`))

(event `SetBoxPos`
  ;[1 1 1] Set Box Pos
  (`SceneComponent.K2_SetWorldLocation` (`self.Box`) (`self.CenterPos`) false false))

(event `Set Center 4`
  ;[1 1 1] Set Center Point
  (set `self.CenterPos` (/ (+ (`self.K2_GetActorLocation` (`GameplayStatics.GetPlayerCharacter` 0)) (`self.K2_GetActorLocation` (`GameplayStatics.GetPlayerCharacter` 1)) (`self.K2_GetActorLocation` (`GameplayStatics.GetPlayerCharacter` 2)) (`self.K2_GetActorLocation` (`GameplayStatics.GetPlayerCharacter` 3))) (4.0 4.0 4.0))))

(event `Set Longest Distance 4`
  (bind _returnvalue (`GameplayStatics.GetPlayerCharacter` 1))
  (bind _returnvalue_2 (`GameplayStatics.GetPlayerCharacter` 2))
  (bind _returnvalue_3 (`GameplayStatics.GetPlayerCharacter` 3))
  (bind _returnvalue_4 (`GameplayStatics.GetPlayerCharacter` 0))
  ;[1 1 1] Take Medium Distance
  (set `self.LongestDistance` (- (`.MaxValue` (`KismetMathLibrary.MaxOfFloatArray` (`|MakeArray` (`self.GetDistanceTo` _returnvalue_4 _returnvalue) (`self.GetDistanceTo` _returnvalue _returnvalue_2) (`self.GetDistanceTo` _returnvalue _returnvalue_3) (`self.GetDistanceTo` _returnvalue_4 _returnvalue_2) (`self.GetDistanceTo` _returnvalue_4 _returnvalue_3) (`self.GetDistanceTo` _returnvalue_2 _returnvalue_3)))) 800.0)))

(event `Set Center 3`
  ;[1 1 1] Set Center Point
  (set `self.CenterPos` (/ (+ (`self.K2_GetActorLocation` (`GameplayStatics.GetPlayerCharacter` 0)) (`self.K2_GetActorLocation` (`GameplayStatics.GetPlayerCharacter` 1)) (`self.K2_GetActorLocation` (`GameplayStatics.GetPlayerCharacter` 2))) (3.0 3.0 3.0))))

(event `Set Center 2`
  ;[1 1 1] Set Center Point
  (set `self.CenterPos` (/ (+ (`self.K2_GetActorLocation` (`GameplayStatics.GetPlayerCharacter` 0)) (`self.K2_GetActorLocation` (`GameplayStatics.GetPlayerCharacter` 1))) (2.0 2.0 2.0))))

(event `Set Longest Distance 3`
  (bind _returnvalue (`GameplayStatics.GetPlayerCharacter` 2))
  (bind _returnvalue_2 (`GameplayStatics.GetPlayerCharacter` 0))
  (bind _returnvalue_3 (`GameplayStatics.GetPlayerCharacter` 1))
  ;[1 1 1] Take Medium Distance
  (set `self.LongestDistance` (- (`.MaxValue` (`KismetMathLibrary.MaxOfFloatArray` (`|MakeArray` (`self.GetDistanceTo` _returnvalue_2 _returnvalue_3) (`self.GetDistanceTo` _returnvalue_3 _returnvalue) (`self.GetDistanceTo` _returnvalue_2 _returnvalue)))) 800.0)))

(event `Set Center 1`
  ;[1 1 1] Set Center Point
  (set `self.CenterPos` (`self.K2_GetActorLocation` (`GameplayStatics.GetPlayerCharacter` 0))))

(event `Set Longest Distance 2`
  ;[1 1 1] Take Medium Distance
  (set `self.LongestDistance` (- (`self.GetDistanceTo` (`GameplayStatics.GetPlayerCharacter` 0) (`GameplayStatics.GetPlayerCharacter` 1)) 800.0)))

(event `Set Longest Distance 1`
  ;[1 1 1] Take Medium Distance
  (set `self.LongestDistance` (- (`self.GetDistanceTo` (`GameplayStatics.GetPlayerCharacter` 0) null) 800.0)))

(event `Set cam Pos`
  ;[0.8229 0.8229 0.8229] Set Cam Pos
  (set `self.CamPosX` (`KismetMathLibrary.FInterpTo` (`self.CamPosX`) (- (.x (`SceneComponent.K2_GetComponentLocation` (`self.Box`))) (`self.XOffset`)) (`self.Delta`) 0.3))
  (set `self.CamPosY` (`KismetMathLibrary.FInterpTo` (`self.CamPosY`) (.y (`SceneComponent.K2_GetComponentLocation` (`self.Box`))) (`self.Delta`) 0.3))
  (`SceneComponent.K2_SetWorldLocation` (`self.SpringArm`) (`KismetMathLibrary.MakeVector` (`self.CamPosX`) (`self.CamPosY`) (.z (`self.CamPosStart`))) false false))

(fn `UserConstructionScript`)